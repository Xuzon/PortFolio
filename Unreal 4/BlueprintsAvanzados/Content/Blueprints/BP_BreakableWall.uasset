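; BP_BreakableWall is a wall actor that cracks in stages each time something bumps it, then destroys itself.
; The SomethingBump event increments BreakLevel and applies the matching entry from the Mats array to the Cube mesh.
; Once BreakLevel runs past the end of Mats, the actor is destroyed, so the material count sets how many hits it takes.
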(event `/Game/Blueprints/Interfaces/BPI_Bumpable.SomethingBump`
  (bind _mats (`self.Mats`))
  (bind _result (`/Engine/EditorBlueprintResources/StandardMacros.IncrementInt` (`self.BreakLevel`))
    (:`  `
      (bind _output_get (set `self.BreakLevel` _result))
      (if (< _output_get (`KismetArrayLibrary.Array_Length` _mats))
        (`PrimitiveComponent.SetMaterial` (`self.Cube`) 0 (`|GetArrayItem` _mats _output_get))
        (else
          (`self.K2_DestroyActor`))))))

(fn `UserConstructionScript`)
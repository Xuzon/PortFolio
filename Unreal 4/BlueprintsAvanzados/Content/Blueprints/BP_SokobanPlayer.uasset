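; Player actor for a Sokoban-style puzzle that creates the HUD on BeginPlay and restarts the current level on R.
; WASD snaps rotation to a direction, then attempts a fixed step through the actor's own Pushable component, which decides whether movement succeeds.
; A successful step fires OnMoved; a blocked one sends a bump message to the actor hit by an eye-height forward line trace.
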(event `Key|R`
  (params (Key :type "Key Structure"))
  ;[1 1 1] Restart Level
  (:`Pressed`
    (bind _returnvalue (`GameplayStatics.GetCurrentLevelName` true))
    (`GameplayStatics.OpenLevel` (`KismetStringLibrary.Conv_StringToName` _returnvalue))))

(event `self.ReceiveBeginPlay`
  ;[1 1 1] Create HUD
  (bind _returnvalue (`|CreateWidget` "/Game/HUD/HUD.HUD_C"))
  (`UserWidget.AddToViewport` _returnvalue 0))

(event `Key|W`
  (params (Key :type "Key Structure"))
  ;[1 1 1] Input
  (:`Pressed`
    (`self.K2_SetActorRotation` (struct))
    (`self.TryMoveForward` 100.0)))

(event `Key|A`
  (params (Key :type "Key Structure"))
  ;[1 1 1] Input
  (:`Pressed`
    (`self.K2_SetActorRotation` (struct :`Yaw` -90.0))
    (`self.TryMoveForward` 100.0)))

(event `Key|S`
  (params (Key :type "Key Structure"))
  ;[1 1 1] Input
  (:`Pressed`
    (`self.K2_SetActorRotation` (struct :`Yaw` 180.0))
    (`self.TryMoveForward` 100.0)))

(event `Key|D`
  (params (Key :type "Key Structure"))
  ;[1 1 1] Input
  (:`Pressed`
    (`self.K2_SetActorRotation` (struct :`Yaw` 90.0))
    (`self.TryMoveForward` 100.0)))

(fn `Damage`)

(fn `MoveTo`
  (params (NewPos :type "Vector Structure"))
  (returns (Moved :type Boolean))
  (bind _pushed (`/Game/Blueprints/Components/Pushable.Push` (`self.Pushable`) NewPos 3))
  (return _pushed))

(fn `TryBump`
  (params (Other :type "Actor Object Reference"))
  (message `/Game/Blueprints/Interfaces/BPI_Bumpable.SomethingBump` Other))

(fn `TryMoveForward`
  (params (Distance :type "Float (double-precision)"))
  (returns (Can :type Boolean))
  (bind _returnvalue (* (`self.GetActorForwardVector`) Distance))
  (bind _returnvalue_2 (+ (`self.K2_GetActorLocation`) (* (`self.GetActorUpVector`) (`self.EyesHeight`))))
  (bind _outhit (`KismetSystemLibrary.LineTraceSingle` _returnvalue_2 (+ _returnvalue_2 _returnvalue) "TraceTypeQuery1"))
  (bind _moved (`self.MoveTo` _returnvalue))
  (if _moved
    (`self.OnMoved`)
    (return true)
    (else
      (`self.TryBump` (`.HitActor` (`GameplayStatics.BreakHitResult` _outhit)))
      (return false))))

(fn `TryPush`
  (params (Other :type "Actor Object Reference") (Direction :type "Vector Structure"))
  (returns (Pushed :type Boolean))
  (bind _returnvalue (`self.GetComponentByClass` Other "/Game/Blueprints/Components/Pushable.Pushable_C"))
  (`/Engine/EditorBlueprintResources/StandardMacros.IsValid` _returnvalue
    (:`Is Valid`
      (bind _pushed (`/Game/Blueprints/Components/Pushable.Push` _returnvalue Direction 2))
      (return _pushed))))

(fn `UserConstructionScript`)
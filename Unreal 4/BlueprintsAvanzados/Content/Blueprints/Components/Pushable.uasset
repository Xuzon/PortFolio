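; Pushable is an actor component that lets its owner be shoved by a direction vector, including chains of adjacent pushables.
; Push spends one point of strength, then line-traces on Visibility along that vector and teleport-style moves the owner, without sweep, if clear.
; A blocking Pushable is pushed recursively with the remaining strength, and the owner moves only if that succeeds.
; EnablePush and DisablePush toggle whether pushes are accepted.
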(fn `DisablePush`
  (set `self.Enabled` false))

(fn `EnablePush`
  (set `self.Enabled` true))

(fn `Push`
  (params (Direction :type "Vector Structure") (PushableStrength :type Integer))
  (returns (Pushed :type Boolean))
  (locals (Dir :type "Vector Structure"))
  (bind _returnvalue (`self.GetOwner`))
  (bind _returnvalue_2 (`Actor.K2_GetActorLocation` _returnvalue))
  (bind _returnvalue_3 (+ (`local.Dir`) _returnvalue_2))
  ;[1 1 1] Am I Enabled
  (if (`self.Enabled`)
    ;[1 1 1] Do not Push if not enough strength
    (bind _result (`/Engine/EditorBlueprintResources/StandardMacros.DecrementInt` PushableStrength)
      (:`  `
        (if (< _result 0)
          (return false)
          (else
            (set `local.Dir` Direction)
            (bind (_outhit _returnvalue_4) (`KismetSystemLibrary.LineTraceSingle` (+ _returnvalue_2 (0.0 0.0 50.0)) (+ _returnvalue_3 (0.0 0.0 50.0)) "TraceTypeQuery1"))
            (if (not (not _returnvalue_4))
              (bind _returnvalue_5 (`Actor.GetComponentByClass` (`.HitActor` (`GameplayStatics.BreakHitResult` _outhit)) "Pushable_C"))
              ;[1 1 1] Maybe I hit another pushable, try to push it
              (`/Engine/EditorBlueprintResources/StandardMacros.IsValid` _returnvalue_5
                (:`Is Valid`
                  (bind _pushed (`self.Push` _returnvalue_5 (`local.Dir`) _result))
                  (if _pushed
                    _
                    (else
                      (return false))))
                (:`Is Not Valid`
                  (return false))))
            ;[1 1 1] Move
            (`Actor.K2_SetActorLocation` _returnvalue _returnvalue_3 false false)
            (return true)))))
    (else
      (return false))))
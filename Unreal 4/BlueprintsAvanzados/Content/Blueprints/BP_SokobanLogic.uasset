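; BP_SokobanLogic tracks move count and puzzle completion for a Sokoban-style box-pushing level.
; On BeginPlay it binds to the player pawn's OnMoved event and counts the level's BP_Box actors.
; Each move increments its own counter and the step total on BP_SokobanInstance.
; OnLandedBox and OnUnlandedBox maintain a landed count; when it matches the box total, pushing is disabled on every box.
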(event `self.ReceiveBeginPlay`
  (`|ExecutionSequence`
    (:`then_0`
      ;[1 1 1] Bind Player to Camera
      (bind _asbp_sokoban_player (cast `/Game/Blueprints/BP_SokobanPlayer` (`GameplayStatics.GetPlayerPawn` 0)))
      (add `/Game/Blueprints/BP_SokobanPlayer.OnMoved` _asbp_sokoban_player (delegate `PlayerMoved`)))
    (:`then_1`
      (bind _outactors (`GameplayStatics.GetAllActorsOfClass` "/Game/Blueprints/BP_Box.BP_Box_C"))
      (set `self.Boxes` (`KismetArrayLibrary.Array_Length` _outactors)))))

(event `PlayerMoved`
  ;[1 1 1] Bind Player to Camera
  (`/Engine/EditorBlueprintResources/StandardMacros.IncrementInt` (`self.NumMovements`)
    (:`  `
      (bind _asbp_sokoban_instance (cast `/Game/Blueprints/BP_SokobanInstance` (`GameplayStatics.GetGameInstance`)))
      (`/Engine/EditorBlueprintResources/StandardMacros.IncrementInt` (`/Game/Blueprints/BP_SokobanInstance.Steps` _asbp_sokoban_instance)))))

(event `OnLandedBox`
  (bind _result (`/Engine/EditorBlueprintResources/StandardMacros.IncrementInt` (`self.LandedBoxes`))
    (:`  `
      (if (== _result (`self.Boxes`))
        (bind _outactors (`GameplayStatics.GetAllActorsOfClass` "/Game/Blueprints/BP_Box.BP_Box_C"))
        (for _array_element _outactors
          (`/Game/Blueprints/Components/Pushable.DisablePush` (`/Game/Blueprints/BP_Box.Pushable` _array_element)))))))

(event `OnUnlandedBox`
  (`/Engine/EditorBlueprintResources/StandardMacros.DecrementInt` (`self.LandedBoxes`)))

(fn `UserConstructionScript`)
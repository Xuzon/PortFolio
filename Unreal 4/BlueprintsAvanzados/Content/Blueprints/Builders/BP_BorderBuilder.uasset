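; BP_BorderBuilder is an actor that builds a rectangular border of tiles, sized by X and Y, when play begins.
; BuildWalls runs two loops, one for the full top and bottom rows and one for the side columns minus the corners.
; SpawnTileAt adds each tile as a Child Actor Component of the Tile class on a 100-unit grid relative to the builder, provided that class is valid.
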(event `self.ReceiveBeginPlay`
  (`self.BuildWalls`))

(fn `BuildWalls`
  (`|ExecutionSequence`
    (:`then_0`
      (for _index (range (`self.X`))
        (`self.SpawnTileAt` _index)
        (`self.SpawnTileAt` _index (- (`self.Y`) 1))))
    (:`then_1`
      (for _index_2 (range 1 (+ (- (`self.Y`) 2) 1))
        (`self.SpawnTileAt` 0 _index_2)
        (`self.SpawnTileAt` (- (`self.X`) 1) _index_2)))))

(fn `SpawnTileAt`
  (params (X :type Integer) (Y :type Integer))
  (if (`KismetSystemLibrary.IsValidClass` (`self.Tile`))
    (bind _returnvalue (`AddComponent|NODE_AddChildActorComponent-0` :`RelativeTransform` (`KismetMathLibrary.Conv_VectorToTransform` (* (`KismetMathLibrary.MakeVector` (`KismetMathLibrary.Conv_IntToDouble` X) (`KismetMathLibrary.Conv_IntToDouble` Y)) 100.0))))
    (`ChildActorComponent.SetChildActorClass` _returnvalue (`self.Tile`))))

(fn `UserConstructionScript`)
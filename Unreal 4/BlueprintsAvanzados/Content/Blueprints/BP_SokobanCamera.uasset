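; Sokoban follow camera that smoothly moves and turns each tick to keep its Target's eye point in view.
; BeginPlay stores the starting offset and distance to the Target.
; RefreshPosition samples points from a natural position toward a last-resort one, taking the first with clear line of sight.
; Visibility traces treat BPI_CameraKindable blockers as see-through and notify them that they are in the way.
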(event `self.ReceiveBeginPlay`
  (bind _target (`self.Target`))
  (`/Engine/EditorBlueprintResources/StandardMacros.IsValid` _target
    (:`Is Valid`
      (`self.CalculateDistance` _target))))

(event `self.ReceiveTick`
  (params (DeltaSeconds :type "Float (single-precision)"))
  (`self.RefreshPosition`)
  (`self.RefreshRotation`))

(fn `CalculateDistance`
  (params (toWho :type "Actor Object Reference"))
  (bind _returnvalue (- (`self.K2_GetActorLocation`) (`self.K2_GetActorLocation` toWho)))
  (set `self.Offset` _returnvalue)
  (set `self.Distance` (`KismetMathLibrary.VSize` _returnvalue))
  (return))

(fn `CanSeeTargetFrom`
  (params (Pos :type "Vector Structure"))
  (returns (ReturnValue :type Boolean))
  (bind (_outhit _returnvalue) (`KismetSystemLibrary.LineTraceSingle` Pos (`self.GetTargetPosition`) "TraceTypeQuery1" false (`|MakeArray` (`self.Target`))))
  (if _returnvalue
    (if (`KismetSystemLibrary.DoesImplementInterface` (`.HitActor` (`GameplayStatics.BreakHitResult` _outhit)) "/Game/Blueprints/Interfaces/BPI_CameraKindable.BPI_CameraKindable_C")
      (message `/Game/Blueprints/Interfaces/BPI_CameraKindable.YouRInMiddle` (`.HitActor` (`GameplayStatics.BreakHitResult` _outhit)))
      (return true)
      (else
        (return false)))
    (else
      (return true))))

(fn `ChangeTargetActor`
  (params (toSet :type "Actor Object Reference"))
  (set `self.Target` toSet)
  (`self.RefreshPosition`)
  (return))

(fn `GetTargetPosition`
  (returns (Pos :type "Vector Structure"))
  (bind _target (`self.Target`))
  (return (+ (`self.K2_GetActorLocation` _target) (* (`self.GetActorUpVector` _target) (`self.TargetEyesHeight`)))))

(fn `RefreshPosition`
  ;[1 1 1] Calculate Selected Position (Maybe you cannot see the player)
  (set `self.SelectedPosition` (`self.GetLastResourcePosition`))
  (for _index (range 11)
    (bind _returnvalue (`KismetMathLibrary.VLerp` (`self.GetNaturalPos`) (`self.GetLastResourcePosition`) (`KismetMathLibrary.NormalizeToRange` (`KismetMathLibrary.Conv_IntToDouble` _index) 0.0 10.0)))
    ;[1 1 1] Try different positions
    (bind _returnvalue_2 (`self.CanSeeTargetFrom` _returnvalue))
    (if _returnvalue_2
      (set `self.SelectedPosition` _returnvalue)
      (break)))
  (`self.K2_SetActorLocation` (`KismetMathLibrary.VLerp` (`self.K2_GetActorLocation`) (`self.SelectedPosition`) (* (`self.TranslationSpeed`) (`GameplayStatics.GetWorldDeltaSeconds`))))
  (return))

(fn `RefreshRotation`
  (`self.K2_SetActorRotation` (`KismetMathLibrary.RLerp` (`self.K2_GetActorRotation`) (`KismetMathLibrary.FindLookAtRotation` (`self.K2_GetActorLocation`) (`self.GetTargetPosition`)) (* (`GameplayStatics.GetWorldDeltaSeconds`) (`self.RotationSpeed`)))))

(fn `UserConstructionScript`)
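; Tile floor builder Blueprint that generates a floor from a text layout when play begins.
; CreateFloor reads the Description string array, treating each string as a row and each character as a tile.
; CodeToClass maps characters to wood, concrete or metal tile classes, falling back to a landing tile.
; CreateTile adds each tile as a child actor component on a 100-unit XY grid.
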(event `self.ReceiveBeginPlay`
  (`self.CreateFloor`))

(fn `CodeToClass`
  (params (Code :type String))
  (returns (ToRet :type "Actor Class Reference"))
  (switch `string` Code
    (:`Default`
      (return "/Game/Blueprints/Tiles/BP_Landing.BP_Landing_C"))
    (:`M`
      (return "/Game/Blueprints/Tiles/BP_WoodTile.BP_WoodTile_C"))
    (:`C`
      (return "/Game/Blueprints/Tiles/BP_ConcreteTile.BP_ConcreteTile_C"))
    (:`L`
      (return "/Game/Blueprints/Tiles/BP_MetalTile.BP_MetalTile_C"))))

(fn `CreateFloor`
  (locals (NString :type Integer) (NChar :type Integer))
  ;[1 1 1] Iterate array
  (for (_array_element _array_index) (`self.Description`)
    (set `local.NString` _array_index)
    ;[1 1 1] Iterate strings
    (for (_array_element_2 _array_index_2) (`KismetStringLibrary.GetCharacterArrayFromString` _array_element)
      (set `local.NChar` _array_index_2)
      ;[1 1 1] Spawn Tile
      (bind _toret (`self.CodeToClass` _array_element_2))
      (`self.CreateTile` (`local.NChar`) (`local.NString`) _toret))))

(fn `CreateTile`
  (params (X :type Integer) (Y :type Integer) (Tile :type "Actor Class Reference"))
  (if (`KismetSystemLibrary.IsValidClass` Tile)
    (bind _returnvalue (`AddComponent|NODE_AddChildActorComponent-0` :`RelativeTransform` (`KismetMathLibrary.Conv_VectorToTransform` (`KismetMathLibrary.MakeVector` (`KismetMathLibrary.Conv_IntToDouble` (* X 100)) (`KismetMathLibrary.Conv_IntToDouble` (* Y 100))))))
    (`ChildActorComponent.SetChildActorClass` _returnvalue Tile)))

(fn `UserConstructionScript`)